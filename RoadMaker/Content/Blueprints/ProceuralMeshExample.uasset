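; An example actor that builds a flat procedural mesh strip in its construction script, with no runtime logic.
; The first quad's corners derive from GridSize and the actor's world location, followed by hardcoded points farther along X.
; A hand-written index list feeds one mesh section without normals or UVs; it repeats the first triangle and leaves the last two vertices unused.
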(fn `UserConstructionScript`
  (locals (Vertices :type "Array of Vector Structure") (Triangles :type "Array of Integer") (HalfGridSize :type "Float (double-precision)" :default 0.0) (Location :type "Vector Structure" :default (0.0 0.0 0.0)))
  (bind _returnvalue (- (`local.Location`) (`KismetMathLibrary.MakeVector` (`local.HalfGridSize`))))
  (bind _returnvalue_2 (+ (`local.Location`) (`KismetMathLibrary.MakeVector` (`local.HalfGridSize`))))
  (set `local.HalfGridSize` (/ (`self.GridSize`) 2.0))
  (set `local.Location` (`self.K2_GetActorLocation`))
  (`KismetArrayLibrary.Array_Append` (`local.Triangles`) (`|MakeArray` 2 0 1 3 2 1 4 2 3 5 4 3 2 0 1))
  (`KismetArrayLibrary.Array_Append` (`local.Vertices`) (`|MakeArray` (- _returnvalue (0.0 25.0 0.0)) (+ _returnvalue (0.0 25.0 0.0)) (- _returnvalue_2 (0.0 25.0 0.0)) (+ _returnvalue_2 (0.0 25.0 0.0)) (550.0 -25.0 0.0) (550.0 25.0 0.0) (650.0 -25.0 0.0) (650.0 25.0 0.0)))
  (`ProceduralMeshComponent.CreateMeshSection_LinearColor` :`self` (`self.ProceduralMesh`) :`Vertices` (`local.Vertices`) :`Triangles` (`local.Triangles`)))