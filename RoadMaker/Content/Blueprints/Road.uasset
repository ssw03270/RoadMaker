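; Road Blueprint that draws a procedural road mesh, starting as a flat disc sized by RoadSize.
; The construction script builds a triangle fan in one-degree steps around a center vertex and applies a dynamic M_Grid material tinted by RoadColor.
; Helper functions append vertices and index-offset triangles, and UpdateRoadSection rebuilds the mesh section from those arrays.
; The Opacity value targets a parameter named "None", and the event graph is empty.
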(event `self.ReceiveTick`
  (params (DeltaSeconds :type "Float (single-precision)")))

(fn `AppendTriangles`
  (params (triangles :type "Array of Integer"))
  (locals (tmp :type "Array of Integer"))
  (for _array_element triangles
    (`KismetArrayLibrary.Array_Add` (`local.tmp`) (+ _array_element (`KismetArrayLibrary.Array_Length` (`self.Vertices`)))))
  (`KismetArrayLibrary.Array_Append` (`self.Triangles`) (`local.tmp`)))

(fn `AppendVertices`
  (params (vertices :type "Array of Vector Structure"))
  (`KismetArrayLibrary.Array_Append` (`self.Vertices`) vertices))

(fn `CreateDefaultSection`
  (locals (HalfRoadSize :type "Float (double-precision)" :default 0.0) (Center :type "Vector Structure" :default (0.0 0.0 0.0)))
  (bind (_center_x _center_y) (`KismetMathLibrary.BreakVector` (`local.Center`)))
  (bind _returnvalue (`KismetArrayLibrary.Array_Length` (`self.Vertices`)))
  (set `local.HalfRoadSize` (/ (`self.RoadSize`) 2.0))
  (bind _output_get (set `local.Center` (0.0 0.0 0.0)))
  (`KismetArrayLibrary.Array_Add` (`self.Vertices`) _output_get)
  (for _index (range 361)
    (`KismetArrayLibrary.Array_Append` (`self.Triangles`) (`|MakeArray` (+ _returnvalue 1) (+ _returnvalue 0) 0))
    (bind _returnvalue_2 (`KismetMathLibrary.Conv_IntToDouble` _index))
    (`KismetArrayLibrary.Array_Append` (`self.Vertices`) (`|MakeArray` (`KismetMathLibrary.MakeVector` (+ (* (`KismetMathLibrary.DegCos` _returnvalue_2) (`local.HalfRoadSize`)) _center_x) (+ _center_y (* (`KismetMathLibrary.DegSin` _returnvalue_2) (`local.HalfRoadSize`)))) :!type "Vector Structure"))))

(fn `CreateMaterialInstance`
  (params (Color :type "LinearColor Structure") (Opacity :type "Float (double-precision)"))
  (returns (MaterialInstance :type "MaterialInstanceDynamic Object Reference"))
  (bind _returnvalue (`KismetMaterialLibrary.CreateDynamicMaterialInstance` "/Game/Contents/Material/M_Grid.M_Grid"))
  (`MaterialInstanceDynamic.SetVectorParameterValue` _returnvalue "Color" Color)
  (`MaterialInstanceDynamic.SetScalarParameterValue` _returnvalue "None" Opacity)
  (return _returnvalue))

(fn `UpdateRoadSection`
  (`ProceduralMeshComponent.CreateMeshSection_LinearColor` :`self` (`self.ProceduralMesh`) :`Vertices` (`self.Vertices`) :`Triangles` (`self.Triangles`)))

(fn `UserConstructionScript`
  (bind _materialinstance (`self.CreateMaterialInstance` (`self.RoadColor`) (`self.Opacity`)))
  (set `self.MaterialInstance` _materialinstance)
  (`self.CreateDefaultSection`)
  (`ProceduralMeshComponent.CreateMeshSection_LinearColor` :`self` (`self.ProceduralMesh`) :`Vertices` (`self.Vertices`) :`Triangles` (`self.Triangles`))
  (`PrimitiveComponent.SetMaterial` (`self.ProceduralMesh`) 0 (`self.MaterialInstance`)))